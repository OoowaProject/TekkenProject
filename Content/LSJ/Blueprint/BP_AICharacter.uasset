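; AI-controlled character Blueprint, judging by its name, for a Tekken 8-style fighter, handling body pushing between characters.
; When its capsule begins overlapping another CPP_Tekken8CharacterParent, it compares that character's X velocity against its own speed.
; Unless the other is faster, both capsules shift by this character's XY movement since PreviousLocation.
; A spine line trace and a facing dot-product check remain as disconnected, unused logic.
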(event OnComponentBeginOverlap(CapsuleComponent)
  (params (OverlappedComponent :type Primitive%20Component%20Object%20Reference) (OtherActor :type Actor%20Object%20Reference) (OtherComp :type Primitive%20Component%20Object%20Reference) (OtherBodyIndex :type Integer) (bFromSweep :type Boolean) (SweepResult :type Hit%20Result%20Structure%20%28by%20ref%29))
  (bind _returnvalue (Transformation|GetActorLocation))
  (bind _previouslocation (Variables|Default|GetpreviousLocation))
  (bind _returnvalue_2 (- _returnvalue _previouslocation))
  (bind (_x _y) (Math|Vector|BreakVector _returnvalue_2))
  (bind _ascpp_tekken_8character_parent (Utilities|Casting|CastToCPP_Tekken8CharacterParent OtherActor))
  (if (not (> (Math|Float|Absolute(Float) (.X (Math|Vector|BreakVector (Variables|/Script/Tekken8.CPP_Tekken8CharacterParent|GetcurrentVelocity _ascpp_tekken_8character_parent)))) (Math|Float|Absolute(Float) (Math|Vector|VectorLength (Variables|Default|GetcurrentVelocity)))))
    (Transformation|AddRelativeLocation (Variables|/Script/Engine.Character|GetCapsuleComponent _ascpp_tekken_8character_parent) (Math|Vector|MakeVector _x _y 0.0) false false)))

(event OnComponentHit(CapsuleComponent)
  (params (HitComponent :type Primitive%20Component%20Object%20Reference) (OtherActor :type Actor%20Object%20Reference) (OtherComp :type Primitive%20Component%20Object%20Reference) (NormalImpulse :type Vector :default "0, 0, 0") (Hit :type Hit%20Result%20Structure%20%28by%20ref%29)))

(event EventBeginPlay)

(event Collision|EventActorBeginOverlap
  (params (OtherActor :type Actor%20Object%20Reference)))

(event EventTick
  (params (DeltaSeconds :type Float%20%28single-precision%29)))

(fn ConstructionScript)