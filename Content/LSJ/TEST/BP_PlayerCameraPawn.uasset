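; BP_PlayerCameraPawn is a test camera pawn that follows the midpoint between two player characters.
; On BeginPlay it stores up to four Characters by their GetAllActorsOfClass order, though only the first two drive the camera.
; Each Tick it moves itself halfway between Player1 and Player2.
; A zoom that sets MainCamera's field of view from their separation is present but never runs.
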(event EventBeginPlay
  ;[1 1 1] 플레이어 변수에 넣기
  (bind _outactors (Actor|GetAllActorsOfClass "/Script/Engine.Character"))
  (for (_array_element _array_index) _outactors
    (switch int _array_index
      (:0
        (Variables|Default|SetPlayer1 _array_element))
      (:1
        (Variables|Default|SetPlayer2 _array_element))
      (:2
        (Variables|Default|SetPlayer2_0 _array_element))
      (:3
        (Variables|Default|SetPlayer2_1 _array_element)))))

(event Collision|EventActorBeginOverlap
  (params (OtherActor :type Actor%20Object%20Reference)))

(event EventTick
  (params (DeltaSeconds :type Float%20%28single-precision%29))
  (bind _player2 (Variables|Default|GetPlayer2))
  (bind _returnvalue (Transformation|GetActorLocation _player2))
  ;[1 1 1] 플레이어와 플레이어 중간 Location
  (Transformation|SetActorLocation (+ (* (- (Transformation|GetActorLocation (Variables|Default|GetPlayer1)) _returnvalue) 0.5) _returnvalue) false false))

(fn ConstructionScript)